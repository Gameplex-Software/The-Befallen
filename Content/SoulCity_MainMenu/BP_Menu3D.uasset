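; BP_Menu3D is a 3D menu actor for the SoulCity main menu that doubles as a camera view target.
; On BeginPlay it shows the mouse cursor, sets game-and-UI input and transitions to itself.
; TransitionTo disables its own collision, enables the destination menu's and blends the player's view to that menu with eased timing, so collision follows the active menu.
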(event Custom|TransitionTo
  (params (DestinationMenu :type BP%20Menu%203D%20Object%20Reference))
  ;[1 1 1] Camera transitions and collision control
  (Collision|SetActorEnableCollision false)
  (Collision|SetActorEnableCollision DestinationMenu true)
  (Game|Player|SetViewTargetwithBlend (Game|GetPlayerController 0) DestinationMenu 2.0 "VTBlend_EaseInOut" 2.0 false))

(event EventBeginPlay
  (bind _self self)
  (Input|SetInputModeGameandUI (Game|GetPlayerController 0) 0 "DoNotLock" true false)
  (Variables|/Script/Engine.PlayerController|SetbShowMouseCursor (Game|GetPlayerController 0) true)
  (CallFunction|Transitionto _self _self))

(fn ConstructionScript)